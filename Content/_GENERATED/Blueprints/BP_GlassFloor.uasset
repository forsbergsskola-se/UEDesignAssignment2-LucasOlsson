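; Glass floor actor that breaks once when any actor overlaps its trigger box.
; The overlap hides and destroys the intact glass, shows the fractured version, then moves a sphere to the overlapping actor's XY, slightly above its own height, and enables its gravity.
; The whole actor destroys itself after a short delay.
; The BreakGlass event is an empty stub.
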(event `BreakGlass`
  (params (Player :type "/Game/_GENERATED/Blueprints/BP_PlayerCharacter Object Reference")))

(event `self.Box.OnComponentBeginOverlap`
  (params (OverlappedComponent :type "PrimitiveComponent Object Reference") (OtherActor :type "Actor Object Reference") (OtherComp :type "PrimitiveComponent Object Reference") (OtherBodyIndex :type Integer) (bFromSweep :type Boolean) (SweepResult :type "HitResult Structure (by ref)"))
  (bind (_returnvalue_x _returnvalue_y) (`KismetMathLibrary.BreakVector` (`self.K2_GetActorLocation` OtherActor)))
  (bind _intactglass (`self.IntactGlass`))
  (bind _sphere (`self.Sphere`))
  (bind (_returnvalue_x_2 _returnvalue_y_2 _returnvalue_z) (`KismetMathLibrary.BreakVector` (`SceneComponent.K2_GetComponentLocation` _sphere)))
  ;[1 1 1] Check if already trigged
  (if (not (`self.AlreadyBroke?`))
    (set `self.AlreadyBroke?` true)
    ;[1 1 1] Removing the visibility and collision from intact glass
    (`SceneComponent.SetVisibility` _intactglass false false)
    (`PrimitiveComponent.SetCollisionEnabled` _intactglass "NoCollision")
    (`SceneComponent.SetVisibility` (`self.FractureGlass`) true false)
    (`ActorComponent.K2_DestroyComponent` (`self.IntactGlass`))
    (`SceneComponent.K2_SetWorldLocation` _sphere (`KismetMathLibrary.MakeVector` _returnvalue_x _returnvalue_y (+ _returnvalue_z 10.0)) false true)
    (`PrimitiveComponent.SetEnableGravity` _sphere true)
    (`KismetSystemLibrary.Delay` 5.0)
    (`self.K2_DestroyActor`)))

(fn `UserConstructionScript`)