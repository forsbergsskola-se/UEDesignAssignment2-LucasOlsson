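; BP_MovableActor is a physics object the player can push along one of two axes.
; X and Y collision overlaps store the player and axis, and enable Tick until the overlap ends.
; Tick compares the player's facing to the mesh axis via a dot-product threshold, toggling the player's push mode when that state changes.
; Starting a push zeroes mesh velocity and plane-constrains its physics to the chosen axis.
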(event `self.Y axis collision.OnComponentBeginOverlap`
  (params (OverlappedComponent :type "PrimitiveComponent Object Reference") (OtherActor :type "Actor Object Reference") (OtherComp :type "PrimitiveComponent Object Reference") (OtherBodyIndex :type Integer) (bFromSweep :type Boolean) (SweepResult :type "HitResult Structure (by ref)"))
  ;[1 1 1] Y axis collision
  (bind _asbp_player_character (cast `/Game/_GENERATED/Blueprints/BP_PlayerCharacter` OtherActor))
  (set `self.Player refe` _asbp_player_character)
  (set `self.IsXAxis` false)
  (`self.EnablePush` true))

(event `EnablePush`
  (params (Enable :type Boolean))
  ;[1 1 1] Push Function
  (if Enable
    (`self.SetActorTickEnabled` true)
    (else
      (`self.SetActorTickEnabled` false)
      (`/Game/_GENERATED/Blueprints/BP_PlayerCharacter.PushMode` (`self.Player refe`) false)
      (set `self.IsPushingEnabled?` false))))

(event `self.Y axis collision.OnComponentEndOverlap`
  (params (OverlappedComponent :type "PrimitiveComponent Object Reference") (OtherActor :type "Actor Object Reference") (OtherComp :type "PrimitiveComponent Object Reference") (OtherBodyIndex :type Integer))
  ;[1 1 1] Y axis collision
  (cast `/Game/_GENERATED/Blueprints/BP_PlayerCharacter` OtherActor)
  (`self.EnablePush` false))

(event `self.ReceiveTick`
  (params (DeltaSeconds :type "Float (single-precision)"))
  (bind _player_refe (`self.Player refe`))
  ;[1 1 1] Push Function
  (if (!= (`self.Check Direction` _player_refe) (`/Game/_GENERATED/Blueprints/BP_PlayerCharacter.IsPushing?` _player_refe))
    (if (`self.IsPushingEnabled?`)
      (`/Game/_GENERATED/Blueprints/BP_PlayerCharacter.PushMode` (`self.Player refe`) true)
      (`PrimitiveComponent.SetAllPhysicsLinearVelocity` (`self.Pushmesh`) (0.0 0.0 0.0) false)
      (if (`self.IsXAxis`)
        (`PrimitiveComponent.SetConstraintMode` (`self.Pushmesh`) "XZPlane")
        (else
          (`PrimitiveComponent.SetConstraintMode` (`self.Pushmesh`) "YZPlane")))
      (else
        (`/Game/_GENERATED/Blueprints/BP_PlayerCharacter.PushMode` (`self.Player refe`) false)
        (`PrimitiveComponent.SetConstraintMode` (`self.Pushmesh`) "None")))))

(event `self.X axis collision.OnComponentBeginOverlap`
  (params (OverlappedComponent :type "PrimitiveComponent Object Reference") (OtherActor :type "Actor Object Reference") (OtherComp :type "PrimitiveComponent Object Reference") (OtherBodyIndex :type Integer) (bFromSweep :type Boolean) (SweepResult :type "HitResult Structure (by ref)"))
  ;[1 1 1] X axis collision
  (bind _asbp_player_character (cast `/Game/_GENERATED/Blueprints/BP_PlayerCharacter` OtherActor))
  (set `self.Player refe` _asbp_player_character)
  (set `self.IsXAxis` true)
  (`self.EnablePush` true))

(event `self.X axis collision.OnComponentEndOverlap`
  (params (OverlappedComponent :type "PrimitiveComponent Object Reference") (OtherActor :type "Actor Object Reference") (OtherComp :type "PrimitiveComponent Object Reference") (OtherBodyIndex :type Integer))
  ;[1 1 1] X axis collision
  (cast `/Game/_GENERATED/Blueprints/BP_PlayerCharacter` OtherActor)
  (`self.EnablePush` false))

(fn `Check Direction`
  (params (Player :type "/Game/_GENERATED/Blueprints/BP_PlayerCharacter Object Reference"))
  (returns (ReturnValue :type Boolean))
  (bind _pushmesh (`self.Pushmesh`))
  (bind _output_get (set `self.IsPushingEnabled?` (> (`KismetMathLibrary.Abs` (`KismetMathLibrary.Dot_VectorVector` (`self.GetActorForwardVector` Player) (select `bool` (`self.IsXAxis`) :`false` (`SceneComponent.GetRightVector` _pushmesh) :`true` (`SceneComponent.GetForwardVector` _pushmesh)))) (`self.KosAngle`))))
  (return _output_get))

(fn `UserConstructionScript`)