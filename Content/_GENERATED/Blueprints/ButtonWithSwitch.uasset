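; Interactable button that opens its matching door once a required switch value is recorded in the GameMode.
; Interact looks up KeyToFind in the Switches map, opens each SwitchDoor whose DoorValue matches ButtonValue and blends the player's view to it.
; A missing key instead plays a timeline that flashes an error material on the button.
; Box overlap shows or removes a "press E" widget and toggles a gate.
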(event `/Game/_GENERATED/Blueprints/InteractInterface.Interact`
  (params (Player :type "/Game/_GENERATED/Blueprints/BP_PlayerCharacter Object Reference"))
  ;[1 1 1] Logic for switch with right button
  (bind _asbp_game_mode (cast `/Game/_GENERATED/Blueprints/BP_GameMode` (`GameplayStatics.GetGameMode`)))
  (bind (_value _returnvalue) (`BlueprintMapLibrary.Map_Find` (`/Game/_GENERATED/Blueprints/BP_GameMode.Switches` _asbp_game_mode) (`self.Key to find`)))
  (if _returnvalue
    (if (>= _value (`self.Required Switch Value`))
      ;[1 1 1] Check for the right door with the right button
      (bind _outactors (`GameplayStatics.GetAllActorsOfClass` "/Game/_GENERATED/Blueprints/SwitchDoor.SwitchDoor_C"))
      (for _array_element _outactors
        (if (== (`/Game/_GENERATED/Blueprints/SwitchDoor.Door Value` _array_element) (`self.Button Value`))
          (`/Game/_GENERATED/Blueprints/SwitchDoor.Open Door` _array_element Player)
          ;[1 1 1] Switching view when open door
          (`PlayerController.SetViewTargetWithBlend` (`GameplayStatics.GetPlayerController` 0) _array_element 0.0 "VTBlend_Linear" 0.0 false))))
    (else
      ;[1 1 1] Player feedback when trying to open the door before activating switch
      (`Timeline|Error_changecolor`
        (:`Update`
          (`PrimitiveComponent.SetMaterial` (`self.StaticMesh`) 1 "/Game/Assets/emmisive_inst_error.emmisive_inst_error")
          (`KismetSystemLibrary.Delay` 0.2)
          (`PrimitiveComponent.SetMaterial` (`self.StaticMesh`) 1 null))))))

(event `self.Box.OnComponentBeginOverlap`
  (params (OverlappedComponent :type "PrimitiveComponent Object Reference") (OtherActor :type "Actor Object Reference") (OtherComp :type "PrimitiveComponent Object Reference") (OtherBodyIndex :type Integer) (bFromSweep :type Boolean) (SweepResult :type "HitResult Structure (by ref)"))
  ;[1 1 1] Trigger widget message
  (if true
    (bind _returnvalue (`|CreateWidget` "/Game/_GENERATED/Blueprints/BP_PressEtoOpen.BP_PressEtoOpen_C"))
    (bind _output_get (set `self.OpenDoor` _returnvalue))
    (`UserWidget.AddToViewport` _output_get 0)
    (`/Engine/EditorBlueprintResources/StandardMacros.Gate` true :!via `Open` :!label _label)))

(event `self.Box.OnComponentEndOverlap`
  (params (OverlappedComponent :type "PrimitiveComponent Object Reference") (OtherActor :type "Actor Object Reference") (OtherComp :type "PrimitiveComponent Object Reference") (OtherBodyIndex :type Integer))
  ;[1 1 1] Trigger widget message
  (`Widget.RemoveFromParent` (stale `self.Box.OnComponentBeginOverlap` _returnvalue))
  (goto _label :!via `Close`))

(fn `UserConstructionScript`)