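; Falling cube trap actor that drops when triggered and ragdolls the player character it hits.
; TriggerTrap turns on physics simulation for the static mesh so it can fall.
; When the Sphere overlaps a BP_PlayerCharacter, it disables player controller input, enables physics on the character mesh and pushes it with a force from the trap actor's velocity scaled by Speed.
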(event `self.Sphere.OnComponentBeginOverlap`
  (params (OverlappedComponent :type "PrimitiveComponent Object Reference") (OtherActor :type "Actor Object Reference") (OtherComp :type "PrimitiveComponent Object Reference") (OtherBodyIndex :type Integer) (bFromSweep :type Boolean) (SweepResult :type "HitResult Structure (by ref)"))
  (bind _returnvalue (`GameplayStatics.GetPlayerController` 0))
  (bind _asbp_player_character (cast `/Game/_GENERATED/Blueprints/BP_PlayerCharacter` OtherActor))
  (`self.DisableInput` _returnvalue _returnvalue)
  (bind _mesh (`Character.Mesh` _asbp_player_character))
  (`PrimitiveComponent.SetSimulatePhysics` _mesh true)
  (`PrimitiveComponent.AddForceAtLocation` _mesh (* (`self.GetVelocity`) (`self.Speed`)) (`SceneComponent.K2_GetComponentLocation` _mesh) "None"))

(event `self.TriggerTrap`
  (`PrimitiveComponent.SetSimulatePhysics` (`self.StaticMesh`) true))

(fn `UserConstructionScript`
  (`parent.UserConstructionScript`))