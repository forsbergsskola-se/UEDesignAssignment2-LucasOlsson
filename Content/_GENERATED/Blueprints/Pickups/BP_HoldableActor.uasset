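; BP_HoldableActor is an interactable pickup actor that the player can grab and hold.
; On Interact it enables physics simulation on its static mesh, then passes itself and the world transform of its GrabLocation component to the player's PickUpHoldable.
; The carrying logic lives on the player; BeginPlay, Tick and the construction script add nothing of their own.
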(event `/Game/_GENERATED/Blueprints/InteractInterface.Interact`
  (params (Player :type "/Game/_GENERATED/Blueprints/BP_PlayerCharacter Object Reference"))
  (`PrimitiveComponent.SetSimulatePhysics` (`self.StaticMesh`) true)
  (`/Game/_GENERATED/Blueprints/BP_PlayerCharacter.PickUpHoldable` Player self (`SceneComponent.K2_GetComponentToWorld` (`self.GrabLocation`))))

(fn `UserConstructionScript`
  (`parent.UserConstructionScript`))