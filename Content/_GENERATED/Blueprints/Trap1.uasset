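; Trap1 is a moving trap that shuttles its static mesh back and forth and destroys any actor that triggers its Hit event.
; On BeginPlay it stores the mesh's relative start transform and scales the Animator timeline's play rate by the travel time.
; The timeline lerps location and rotation toward the Destination offset, and a FlipFlop on Finished alternates reverse and forward play for an endless loop.
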(event `self.ReceiveBeginPlay`
  (bind (_returnvalue_location _returnvalue_rotation) (`KismetMathLibrary.BreakTransform` (`SceneComponent.GetRelativeTransform` (`self.StaticMesh`))))
  ;[1 1 1] Store Start Position
  (set `self.StartPos` _returnvalue_location)
  (set `self.StartRot` _returnvalue_rotation)
  (`TimelineComponent.SetPlayRate` (`self.Animator`) (/ 1.0 (`self.TravelTimeInSeconds`)))
  (`self.Move Trap`))

(event `Move Trap`
  (bind (_destination_location _destination_rotation) (`KismetMathLibrary.BreakTransform` (`self.Destination`)))
  (bind _startpos (`self.StartPos`))
  (bind _startrot (`self.StartRot`))
  (bind (_direction _alpha) (`Timeline|Animator` :!label _label)
    (:`Update`
      (set `self.Lerp Alpha` _alpha)
      ;[1 1 1] Move the platform
      (`SceneComponent.K2_SetRelativeLocationAndRotation` (`self.StaticMesh`) (`KismetMathLibrary.VLerp` _startpos (+ _startpos _destination_location) (`self.Lerp Alpha`)) (`KismetMathLibrary.RLerp` _startrot (`KismetMathLibrary.ComposeRotators` _startrot _destination_rotation) (`self.Lerp Alpha`)) false false))
    (:`Finished`
      ;[1 1 1] Pause and Determine next action
      (`/Engine/EditorBlueprintResources/StandardMacros.FlipFlop`
        (:`A`
          (`self.Reverse Movement`))
        (:`B`
          (`self.Move Trap`))))))

(event `Reverse Movement`
  (goto _label :!via `Reverse`))

(event `self.ReceiveHit`
  (params (MyComp :type "PrimitiveComponent Object Reference") (Other :type "Actor Object Reference") (OtherComp :type "PrimitiveComponent Object Reference") (bSelfMoved :type Boolean) (HitLocation :type "Vector Structure") (HitNormal :type "Vector Structure") (NormalImpulse :type "Vector Structure") (Hit :type "HitResult Structure (by ref)"))
  (`self.K2_DestroyActor` Other))

(fn `UserConstructionScript`)