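; Player character test Blueprint with forward teleport, left-hand physics grabbing and a cone-collecting win check.
; Teleport line-traces ahead, moves to the hit or maximum range between camera FOV zoom timelines, then locks out on a timer cooldown.
; A physics handle follows the left hand each Tick, while pickup events tally two cone types and print the win.
; BeginPlay adds an energy widget and stores the respawn transform; stamina cooldown events are never called here.
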(event `New Teleport Cooldown`
  (if (`self.Allow Teleport`)
    (bind _output_get (set `self.Stamina` (`self.Teleport Cost`)))
    (if (== _output_get 0.0)
      (set `self.Allow Teleport` false)
      (else
        (`KismetSystemLibrary.Delay` 0.01)
        (`self.New Teleport Cooldown`)))))

(event `New Clear Teleport Cooldown`
  (if (`self.Allow Teleport`)
    _
    (elif (not (== (`self.Stamina`) (`self.Desired Stamina`)))
      (set `self.Stamina` (`KismetMathLibrary.FClamp` (+ (`self.Stamina`) 0.5) 0.0 (`self.Max Stamina`)))
      (`KismetSystemLibrary.Delay` 0.01))))

(event `Start Teleport Cooldown`
  ;[1 1 1] Teleport Cooldown logic
  (set `self.Allow Teleport` false)
  (`KismetSystemLibrary.K2_SetTimerDelegate` (delegate `Clear Teleport Cooldown`) 3.0))

(event `Clear Teleport Cooldown`
  ;[1 1 1] Teleport Cooldown logic
  (set `self.Allow Teleport` true))

(event `InputAction|Teleportation`
  (params (Key :type "Key Structure"))
  (bind (_outlocation _outrotation) (`self.GetActorEyesViewPoint`))
  (bind _sphere (`self.Sphere`))
  (bind _returnvalue (`SceneComponent.K2_GetComponentLocation` _sphere))
  (bind _returnvalue_2 (+ _returnvalue (* (`SceneComponent.GetForwardVector` _sphere) 600.0)))
  ;[1 1 1] Teleportation Logic
  (:`Pressed`
    (if (`self.Allow Teleport`)
      (bind (_outhit _returnvalue_3) (`KismetSystemLibrary.LineTraceSingle` _returnvalue _returnvalue_2 "TraceTypeQuery1" true))
      (if _returnvalue_3
        (`self.Start Teleport Cooldown`)
        (bind (_direction _alpha) (`Timeline|Teleport` :!via `PlayFromStart`)
          (:`Update`
            (`CameraComponent.SetFieldOfView` (`self.Camera`) (`KismetMathLibrary.Lerp` 90.0 60.0 _alpha)))
          (:`Finished`
            (`self.K2_TeleportTo` (`.Location` (`GameplayStatics.BreakHitResult` _outhit)) _outrotation)
            (bind (_direction_2 _alpha_2) (`Timeline|Timeline_0` :!via `ReverseFromEnd`)
              (:`Update`
                (`CameraComponent.SetFieldOfView` (`self.Camera`) (`KismetMathLibrary.Lerp` 90.0 60.0 _alpha_2))))))
        (else
          (`self.Start Teleport Cooldown`)
          (bind (_direction_3 _alpha_3) (`Timeline|Timeline_1` :!via `PlayFromStart`)
            (:`Update`
              (`CameraComponent.SetFieldOfView` (`self.Camera`) (`KismetMathLibrary.Lerp` 90.0 60.0 _alpha_3)))
            (:`Finished`
              (`self.K2_TeleportTo` _returnvalue_2 _outrotation)
              (bind (_direction_4 _alpha_4) (`Timeline|Timeline_2` :!via `ReverseFromEnd`)
                (:`Update`
                  (`CameraComponent.SetFieldOfView` (`self.Camera`) (`KismetMathLibrary.Lerp` 90.0 60.0 _alpha_4)))))))))))

(event `InputAction|OpenDoor`
  (params (Key :type "Key Structure"))
  ;[1 1 1] Interact with interactable objects
)

(event `PickUpHoldable`
  (params (Holdable :type "/Game/_GENERATED/Blueprints/Pickups/BP_HoldableActor Object Reference") (GrabLocation :type "Transform Structure"))
  (if (not (`self.isHoldingLeftHand`))
    (bind _asprimitive_component (cast `PrimitiveComponent` (`Actor.RootComponent` Holdable)))
    (`PhysicsHandleComponent.GrabComponentAtLocationWithRotation` (`self.LeftPhysicsHandle`) _asprimitive_component "None" (`KismetMathLibrary.TransformLocation` GrabLocation) (`KismetMathLibrary.TransformRotation` GrabLocation))
    (set `self.isHoldingLeftHand` true)))

(event `self.ReceiveDestroyed`
  ;[1 1 1] Respawn Logic
)

(event `self.ReceiveTick`
  (params (DeltaSeconds :type "Float (single-precision)"))
  (bind _lefthandphysics (`self.LeftHandPhysics`))
  (`KismetSystemLibrary.PrintString` (`KismetStringLibrary.Conv_IntToString` (`self.Cones`)) true true (struct :`G` 0.66 :`B` 1.0 :`A` 1.0) 0.0 "ConeKey")
  (`KismetSystemLibrary.PrintString` (`KismetStringLibrary.Conv_IntToString` (`self.RedCones`)) true true (struct :`G` 0.66 :`B` 1.0 :`A` 1.0) 0.0 "RedCones")
  (if (`self.isHoldingLeftHand`)
    (`PrimitiveComponent.WakeRigidBody` (`PhysicsHandleComponent.GetGrabbedComponent` (`self.LeftPhysicsHandle`)) "None")
    (`PhysicsHandleComponent.SetTargetLocationAndRotation` (`self.LeftPhysicsHandle`) (`SceneComponent.K2_GetComponentLocation` _lefthandphysics) (`SceneComponent.K2_GetComponentRotation` _lefthandphysics))))

(event `self.ReceiveBeginPlay`
  ;[1 1 1] Showing Teleport cooldown from start
  (bind _returnvalue (`|CreateWidget` "/Game/_GENERATED/Blueprints/EnergyWidget.EnergyWidget_C"))
  (`UserWidget.AddToViewport` _returnvalue 0)
  ;[1 1 1] Respawn logic
  (bind _asbp_game_mode (cast `/Game/_GENERATED/Blueprints/BP_GameMode` (`GameplayStatics.GetGameMode`)))
  (set `/Game/_GENERATED/Blueprints/BP_GameMode.Respawn Transform` (`self.GetTransform`) _asbp_game_mode))

(event `Add Pickup`
  (params (NumberOfItems :type Integer :default 1))
  ;[1 1 1] Collectible win condition
  (set `self.Cones` (+ (`self.Cones`) NumberOfItems))
  (`self.OnCollectableAdded` :!label _label))

(event `Add Pickup RedCones`
  (params (NumberOfRedCones :type Integer))
  ;[1 1 1] Collectible win condition
  (set `self.RedCones` (+ (`self.RedCones`) NumberOfRedCones))
  (goto _label))

(event `OnCollectableAdded`
  ;[1 1 1] Collectible win condition
  (if (and (>= (`self.Cones`) (`self.ConesNeeded`)) (>= (`self.RedCones`) (`self.RedConesNeeded`)))
    (`KismetSystemLibrary.PrintString` "You Win")))

(fn `UserConstructionScript`)