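; SwitchDoor is a door actor whose OpenDoor and CloseDoor events animate its Sphere component, then return the camera to the supplied Player.
; Each event plays its own timeline to lerp relative location and rotation by the Destination offset.
; Opening starts from StartPos, while closing starts from ReturnPos but applies the same offset and StartRot.
; When either timeline finishes, it waits CameraDelay before blending the view target to Player.
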(event `Open Door`
  (params (Player :type "/Game/_GENERATED/Blueprints/BP_PlayerCharacter Object Reference"))
  (bind _startrot (`self.StartRot`))
  (bind (_destination_location _destination_rotation) (`KismetMathLibrary.BreakTransform` (`self.Destination`)))
  (bind _startpos (`self.StartPos`))
  (`KismetSystemLibrary.Delay` 0.0)
  (`KismetSystemLibrary.PrintString` "Start Ipen mechanic")
  (bind (_direction _alpha) (`Timeline|Open Door T`)
    (:`Update`
      (set `self.Lerp Alpha` _alpha)
      ;[1 1 1] Open the door
      (`SceneComponent.K2_SetRelativeLocationAndRotation` (`self.Sphere`) (`KismetMathLibrary.VLerp` _startpos (+ _startpos _destination_location) (`self.Lerp Alpha`)) (`KismetMathLibrary.RLerp` _startrot (`KismetMathLibrary.ComposeRotators` _startrot _destination_rotation) (`self.Lerp Alpha`)) false false))
    (:`Finished`
      ;[1 1 1] Camera Switch
      (`KismetSystemLibrary.Delay` (`self.CameraDelay`))
      (`PlayerController.SetViewTargetWithBlend` (`GameplayStatics.GetPlayerController` 0) Player 0.0 "VTBlend_Linear" 0.0 false))))

(event `Close Door`
  (params (Player :type "/Game/_GENERATED/Blueprints/BP_PlayerCharacter Object Reference"))
  (bind _returnpos (`self.returnPos`))
  (bind (_destination_location _destination_rotation) (`KismetMathLibrary.BreakTransform` (`self.Destination`)))
  (bind _startrot (`self.StartRot`))
  (`KismetSystemLibrary.Delay` 0.0)
  (`KismetSystemLibrary.PrintString` "Start Ipen mechanic")
  (bind (_direction _alpha) (`Timeline|Timeline_0`)
    (:`Update`
      (set `self.Lerp Alpha` _alpha)
      ;[1 1 1] Open the door
      (`SceneComponent.K2_SetRelativeLocationAndRotation` (`self.Sphere`) (`KismetMathLibrary.VLerp` _returnpos (+ _returnpos _destination_location) (`self.Lerp Alpha`)) (`KismetMathLibrary.RLerp` _startrot (`KismetMathLibrary.ComposeRotators` _startrot _destination_rotation) (`self.Lerp Alpha`)) false false))
    (:`Finished`
      ;[1 1 1] Camera Switch
      (`KismetSystemLibrary.Delay` (`self.CameraDelay`))
      (`PlayerController.SetViewTargetWithBlend` (`GameplayStatics.GetPlayerController` 0) Player 0.0 "VTBlend_Linear" 0.0 false))))

(fn `UserConstructionScript`)